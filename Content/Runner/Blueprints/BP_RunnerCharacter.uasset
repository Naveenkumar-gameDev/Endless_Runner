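; Player character for a three-lane endless runner, loading the saved skin on BeginPlay.
; Once the game starts, Tick drives it forward and interpolates Y toward the lane chosen by swipe or key events.
; It jumps, slides via montages, drops fast mid-air, and ragdolls into the game-over screen on death.
; Timed magnet and jump-boost powers add fading HUD slots; speed can increment or be debug-toggled.
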(event Custom|Death
  (bind _gamemode_ref (Variables|Default|GetGameMode_Ref))
  (bind _gamemode_ref_2 (Variables|Default|GetGameMode_Ref))
  (bind _mesh (Variables|Character|GetMesh))
  (bind _audioplayer (Variables|/Game/Runner/Blueprints/BP_RunnerGameMode.BP_RunnerGameMode_C|GetAudioPlayer _gamemode_ref_2))
  (bind _audiocomponent (Variables|/Script/Engine.AmbientSound|GetAudioComponent _audioplayer))
  (Audio|Components|Audio|SetSound _audiocomponent "/Game/Runner/Audios/game_over_Sound.game_over_Sound")
  (Audio|Components|Audio|Play _audiocomponent 0.0)
  (Pawn|Components|CharacterMovement|DisableMovement (Variables|Character|GetCharacterMovement))
  (Input|DisableInput 0)
  (Physics|SetSimulatePhysics _mesh true)
  (Collision|SetCollisionProfileName _mesh "ragdoll" true :!class /Script/Engine.PrimitiveComponent)
  (bind _returnvalue (UserInterface|CreateWidget "/Game/Runner/Blueprints/HUD/WB_GameOverScreen.WB_GameOverScreen_C" 0 (Variables|/Game/Runner/Blueprints/BP_RunnerGameMode.BP_RunnerGameMode_C|GetCoins _gamemode_ref) (Variables|/Game/Runner/Blueprints/BP_RunnerGameMode.BP_RunnerGameMode_C|GetPlayer_Score _gamemode_ref)))
  (UserInterface|Viewport|AddtoViewport _returnvalue 0)
  (Variables|Default|SetisDead true))

(event Custom|Sliding
  (if (Variables|Default|GetCanSlide)
    (Variables|Default|SetCanSlide false)
    (Animation|Montage|PlayMontage (Variables|Character|GetMesh) "/Game/Runner/Animations/Sliding_new_Montage.Sliding_new_Montage"
      (:OnCompleted
        (Variables|Default|SetCanSlide true)))))

(event Custom|Swip_Up
  (if (Variables|Default|GetCanSlide)
    (Character|Jump)
    (else
      (Variables|Default|SetCanSlide true)
      (Variables|Default|SetIsSliding false)
      (Animation|Montage|PlayMontage (Variables|Character|GetMesh) "/Game/Runner/Animations/Sliding_GetUp_Montage.Sliding_GetUp_Montage" 1.5
        (:OnCompleted
          (Character|Jump))))))

(event Custom|Activate%20Magnet%20Power
  ;[0.15 0.15 0.15 0.5] Magnet Power
  (bind _returnvalue (UserInterface|CreateWidget "/Game/Runner/Blueprints/HUD/WB_PowerUp_Slot.WB_PowerUp_Slot_C"))
  (Class|UniformGridPanel|AddChildtoUniformGrid (Variables|/Game/Runner/Blueprints/HUD/HUD_Player.HUD_Player_C|GetPowerUpGrid (Variables|Default|GetHUD_Player_Ref)) _returnvalue)
  (Collision|SetCollisionEnabled (Variables|Default|GetMagnetCollision) "QueryOnly")
  (Variables|Default|SetIsMagnetEnable true)
  (Utilities|FlowControl|Delay 1e+01)
  (UserInterface|Animation|PlayAnimation _returnvalue (Variables|/Game/Runner/Blueprints/HUD/WB_PowerUp_Slot.WB_PowerUp_Slot_C|GetFadeAnim _returnvalue) 0.0 1 "Forward" 1.0 false)
  (Utilities|FlowControl|Delay 5.0)
  (Variables|Default|SetIsMagnetEnable false)
  (Collision|SetCollisionEnabled (Variables|Default|GetMagnetCollision) "QueryOnly"))

(event Custom|Activate%20Jumb%20Power
  ;[0.15 0.15 0.15 0.5] JumpBoost Power
  (Variables|Default|SetIsJumbBoostEnable true)
  (bind _returnvalue (UserInterface|CreateWidget "/Game/Runner/Blueprints/HUD/WB_PowerUp_Slot.WB_PowerUp_Slot_C" 0 1))
  (Class|UniformGridPanel|AddChildtoUniformGrid (Variables|/Game/Runner/Blueprints/HUD/HUD_Player.HUD_Player_C|GetPowerUpGrid (Variables|Default|GetHUD_Player_Ref)) _returnvalue 1)
  (Variables|/Script/Engine.CharacterMovementComponent|SetJumpZVelocity (Variables|Character|GetCharacterMovement) 1.2e+03)
  (Utilities|FlowControl|Delay 1e+01)
  (UserInterface|Animation|PlayAnimation _returnvalue (Variables|/Game/Runner/Blueprints/HUD/WB_PowerUp_Slot.WB_PowerUp_Slot_C|GetFadeAnim _returnvalue) 0.0 1 "Forward" 1.0 false)
  (Utilities|FlowControl|Delay 5.0)
  (Variables|/Script/Engine.CharacterMovementComponent|SetJumpZVelocity (Variables|Character|GetCharacterMovement) 9e+02)
  (Variables|Default|SetIsJumbBoostEnable false))

(event Custom|Start
  (bind _returnvalue (Game|SpawnActorfromClass "/Game/Runner/Blueprints/Others/BP_PlayerCamera.BP_PlayerCamera_C" (Transformation|GetWorldTransform (Variables|Default|GetCameraSpawnPoint)) "Undefined" "MultiplyWithRoot" 0 self 0))
  (Game|Player|SetViewTargetwithBlend (Game|GetPlayerController 0) _returnvalue 1.0 "VTBlend_Linear" 0.0 false))

(event Custom|Swip_Down
  (bind _charactermovement (Variables|Character|GetCharacterMovement))
  (if (AI|Components|NavMovement|IsFalling (Variables|Character|GetCharacterMovement))
    (if (Variables|Default|GetIsJumbBoostEnable)
      (Physics|AddImpulse _charactermovement (Math|Vector|MakeVector 0.0 0.0 -1e+05) false)
      (else
        (Physics|AddImpulse _charactermovement (Math|Vector|MakeVector 0.0 0.0 -5e+04) false)))
    (else
      (CallFunction|Sliding))))

(event Custom|Swip_left
  (Variables|Default|SetCurrentLane (Math|Integer|Clamp(Integer) (- (Variables|Default|GetCurrentLane) 1) 0 2))
  (Variables|Default|SetTargetY (* (- (Variables|Default|GetCurrentLane) 1) (Variables|Default|GetLaneOffSet))))

(event Custom|Swip_Right
  (Variables|Default|SetCurrentLane (Math|Integer|Clamp(Integer) (+ (Variables|Default|GetCurrentLane) 1) 0 2))
  (Variables|Default|SetTargetY (* (- (Variables|Default|GetCurrentLane) 1) (Variables|Default|GetLaneOffSet))))

(event EventBeginPlay
  (bind _returnvalue (Actor|GetActorOfClass "/Game/Runner/Blueprints/BP_RunnerGameMode.BP_RunnerGameMode_C"))
  (Variables|Default|SetGameMode_Ref _returnvalue)
  (bind _returnvalue_2 (SaveGame|DoesSaveGameExist "saveGame"))
  (if _returnvalue_2
    (bind _returnvalue_3 (SaveGame|LoadGamefromSlot "savegame"))
    (bind _asbp_save_game (Utilities|Casting|CastToBP_SaveGame _returnvalue_3))
    (bind _output_get (Variables|/Game/Runner/Blueprints/BP_RunnerGameMode.BP_RunnerGameMode_C|SetSaveGame_Ref (Variables|Default|GetGameMode_Ref) _asbp_save_game))
    (Components|SkeletalMesh|SetSkeletalMeshAsset (Variables|Character|GetMesh) (.character (Utilities|Array|Get(acopy) (Variables|/Game/Runner/Blueprints/BP_SaveGame.BP_SaveGame_C|GetCharacterData _output_get) (Variables|/Game/Runner/Blueprints/BP_SaveGame.BP_SaveGame_C|GetCurrentCharacterCount _output_get))))
    (Variables|/Game/Runner/Blueprints/BP_RunnerGameMode.BP_RunnerGameMode_C|SetSelectCharacterCount (Variables|Default|GetGameMode_Ref) (Variables|/Game/Runner/Blueprints/BP_SaveGame.BP_SaveGame_C|GetCurrentCharacterCount (Variables|/Game/Runner/Blueprints/BP_RunnerGameMode.BP_RunnerGameMode_C|GetSaveGame_Ref (Variables|Default|GetGameMode_Ref))))))

(event EventTick
  (params (DeltaSeconds :type Float%20%28single-precision%29))
  (if (Variables|/Game/Runner/Blueprints/BP_RunnerGameMode.BP_RunnerGameMode_C|GetIsGameStarted (Variables|Default|GetGameMode_Ref))
    (Pawn|Input|AddMovementInput "1.000000,0.000000,0.000000" 1.0 false)
    (Transformation|SetActorLocation (CallFunction|GetSwitchDistance DeltaSeconds) false false)))

(event Input|ActionEvents|InputActionMoveDown
  (params (Key :type Key%20Structure :default "None"))
  (bind _charactermovement (Variables|Character|GetCharacterMovement))
  (:Pressed
    (if (AI|Components|NavMovement|IsFalling (Variables|Character|GetCharacterMovement))
      (if (Variables|Default|GetIsJumbBoostEnable)
        (Physics|AddImpulse _charactermovement (Math|Vector|MakeVector 0.0 0.0 -1e+05) false)
        (else
          (Physics|AddImpulse _charactermovement (Math|Vector|MakeVector 0.0 0.0 -5e+04) false)))
      (else
        (CallFunction|Sliding)))))

(event Input|ActionEvents|InputActionMoveUp
  (params (Key :type Key%20Structure :default "None"))
  (:Pressed
    (if (Variables|Default|GetCanSlide)
      (Character|Jump)
      (else
        (Variables|Default|SetCanSlide true)
        (Variables|Default|SetIsSliding false)
        (Animation|Montage|PlayMontage (Variables|Character|GetMesh) "/Game/Runner/Animations/Sliding_GetUp_Montage.Sliding_GetUp_Montage" 1.5
          (:OnCompleted
            (Character|Jump)))))))

(event Input|ActionEvents|InputActionMoveLeft
  (params (Key :type Key%20Structure :default "None"))
  (:Pressed
    (Variables|Default|SetCurrentLane (Math|Integer|Clamp(Integer) (- (Variables|Default|GetCurrentLane) 1) 0 2))
    (Variables|Default|SetTargetY (* (- (Variables|Default|GetCurrentLane) 1) (Variables|Default|GetLaneOffSet)))))

(event Input|ActionEvents|InputActionMoveRight
  (params (Key :type Key%20Structure :default "None"))
  (:Pressed
    (Variables|Default|SetCurrentLane (Math|Integer|Clamp(Integer) (+ (Variables|Default|GetCurrentLane) 1) 0 2))
    (Variables|Default|SetTargetY (* (- (Variables|Default|GetCurrentLane) 1) (Variables|Default|GetLaneOffSet)))))

(event Custom|DoubleClick
  (Utilities|FlowControl|FlipFlop
    (:A
      (Variables|Default|SetOldPlayerSpeed (Variables|/Script/Engine.CharacterMovementComponent|GetMaxWalkSpeed (Variables|Character|GetCharacterMovement)))
      (Variables|/Script/Engine.CharacterMovementComponent|SetMaxWalkSpeed (Variables|Character|GetCharacterMovement) 1.5e+03))
    (:B
      (Variables|/Script/Engine.CharacterMovementComponent|SetMaxWalkSpeed (Variables|Character|GetCharacterMovement) (Variables|Default|GetOldPlayerSpeed)))))

(event Input|KeyboardEvents|1
  (params (Key :type Key%20Structure))
  (:Pressed
    (Utilities|FlowControl|FlipFlop
      (:A
        (Variables|Default|SetOldPlayerSpeed (Variables|/Script/Engine.CharacterMovementComponent|GetMaxWalkSpeed (Variables|Character|GetCharacterMovement)))
        (Variables|/Script/Engine.CharacterMovementComponent|SetMaxWalkSpeed (Variables|Character|GetCharacterMovement) 1.5e+03))
      (:B
        (Variables|/Script/Engine.CharacterMovementComponent|SetMaxWalkSpeed (Variables|Character|GetCharacterMovement) (Variables|Default|GetOldPlayerSpeed))))))

(fn ConstructionScript)

(fn AddWalkSpeed
  (bind _charactermovement (Variables|Character|GetCharacterMovement))
  (bind _maxwalkspeed (Variables|/Script/Engine.CharacterMovementComponent|GetMaxWalkSpeed _charactermovement))
  (if (<= (Variables|/Script/Engine.CharacterMovementComponent|GetMaxWalkSpeed (Variables|Character|GetCharacterMovement)) 1.5e+03)
    (Math|Float|IncrementFloat _maxwalkspeed
      (:%20%20
        (Math|Float|IncrementFloat _maxwalkspeed)))
    (else
      (Math|Float|IncrementFloat (Variables|Default|GetOldPlayerSpeed)
        (:%20%20
          (Math|Float|IncrementFloat (Variables|Default|GetOldPlayerSpeed)))))))

(fn GetSwitchDistance
  (params (Delta :type Float%20%28double-precision%29))
  (bind _returnvalue (Transformation|GetActorLocation))
  (return (Math|Vector|MakeVector (.x _returnvalue) (Math|Interpolation|FInterpTo (.y _returnvalue) (Variables|Default|GetTargetY) Delta 3.0) (.z _returnvalue))))