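; Cheat manager for the Runner game, providing debug commands that edit the saved progress.
; ClearData deletes an existing save slot and writes a fresh BP_SaveGame in its place, printing confirmation even when no save exists.
; AddCoins loads the save, sets TotalCoins to a fixed amount rather than incrementing it, and saves it back.
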(fn ClearData
  (bind _returnvalue (SaveGame|DoesSaveGameExist "savegame"))
  (if _returnvalue
    (SaveGame|DeleteGameinSlot "saveGame")
    (bind _returnvalue_2 (SaveGame|CreateSaveGameObject "/Game/Runner/Blueprints/BP_SaveGame.BP_SaveGame_C"))
    (bind _asbp_save_game (Utilities|Casting|CastToBP_SaveGame _returnvalue_2))
    (SaveGame|SaveGametoSlot _asbp_save_game "Savegame")
    (Development|PrintString "Data Cleared" true true "(R=1.000000,G=0.933375,B=0.114583,A=1.000000)")
    (else
      (Development|PrintString "Data Cleared" true true "(R=1.000000,G=0.933375,B=0.114583,A=1.000000)"))))

(fn AddCoins
  (bind _returnvalue (SaveGame|LoadGamefromSlot "SaveGame"))
  (bind _asbp_save_game (Utilities|Casting|CastToBP_SaveGame _returnvalue))
  (Variables|/Game/Runner/Blueprints/BP_SaveGame.BP_SaveGame_C|SetTotal%20Coins _asbp_save_game 5000)
  (SaveGame|SaveGametoSlot _asbp_save_game "SaveGame")
  (Development|PrintString "Coin Added" true true "(R=1.000000,G=0.933375,B=0.114583,A=1.000000)"))