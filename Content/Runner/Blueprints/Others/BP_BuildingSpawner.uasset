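; Building spawner for the runner game that lays a chain of random buildings along one side.
; On BeginPlay it registers itself in BP_RunnerGameMode's SpawnBuildingRef array and takes its root transform as the first spawn location.
; Each SpawnBuilding call spawns one of three building Blueprints, then stores that building's SpawnPoint transform for the next one.
; When IsLeft is set, the new building is mirrored through negative Y scale.
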(event EventBeginPlay
  (bind _returnvalue (Actor|GetActorOfClass "/Game/Runner/Blueprints/BP_RunnerGameMode.BP_RunnerGameMode_C"))
  (Utilities|Array|Add (Variables|/Game/Runner/Blueprints/BP_RunnerGameMode.BP_RunnerGameMode_C|GetSpawnBuilding_Ref _returnvalue) self)
  (Variables|Default|SetSpawnLocation (Transformation|GetRelativeTransform (Variables|Default|GetDefaultSceneRoot))))

(event Collision|EventActorBeginOverlap
  (params (OtherActor :type Actor%20Object%20Reference)))

(event EventTick
  (params (DeltaSeconds :type Float%20%28single-precision%29)))

(fn ConstructionScript)

(fn SpawnBuilding
  (switch int (Math|Random|RandomIntegerinRange 0 2)
    (:0
      (bind _returnvalue (Game|SpawnActorfromClass "/Game/Runner/Models/BP_Building_01.BP_Building_01_C" (Variables|Default|GetSpawnLocation) "Undefined" "MultiplyWithRoot" 0 0))
      (Variables|Default|SetBuilding _returnvalue)
      (Variables|Default|SetSpawnLocation (Transformation|GetWorldTransform (Variables|/Game/Runner/Models/BP_Building_01.BP_Building_01_C|GetSpawnPoint _returnvalue))))
    (:1
      (bind _returnvalue_2 (Game|SpawnActorfromClass "/Game/Runner/Models/BP_Building_02.BP_Building_02_C" (Variables|Default|GetSpawnLocation) "Undefined" "MultiplyWithRoot" 0 0))
      (Variables|Default|SetBuilding _returnvalue_2)
      (Variables|Default|SetSpawnLocation (Transformation|GetWorldTransform (Variables|/Game/Runner/Models/BP_Building_02.BP_Building_02_C|GetSpawnPoint _returnvalue_2))))
    (:2
      (bind _returnvalue_3 (Game|SpawnActorfromClass "/Game/Runner/Models/BP_Building_03.BP_Building_03_C" (Variables|Default|GetSpawnLocation) "Undefined" "MultiplyWithRoot" 0 0))
      (Variables|Default|SetBuilding _returnvalue_3)
      (Variables|Default|SetSpawnLocation (Transformation|GetWorldTransform (Variables|/Game/Runner/Models/BP_Building_03.BP_Building_03_C|GetSpawnPoint _returnvalue_3)))))
  (if (Variables|Default|GetIsLeft)
    (Transformation|SetActorScale3D (Variables|Default|GetBuilding) "1.000000,-1.000000,1.000000")))