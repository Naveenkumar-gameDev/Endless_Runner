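; Player controller for a runner game that turns touch input into swipe and double-tap commands on the runner character.
; On BeginPlay it caches the character and game mode.
; While the game has started, touch movement beyond a threshold from the press point triggers a four-way swipe call and deactivates tracking.
; Touch releases increment a tap counter, with a short Delay before reset acting as the double-tap window.
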(event EventBeginPlay
  (bind _asbp_runner_character (Utilities|Casting|CastToBP_RunnerCharacter (Game|GetPlayerCharacter 0)))
  (Variables|Default|SetPlayerRef _asbp_runner_character)
  (bind _asbp_runner_game_mode (Utilities|Casting|CastToBP_RunnerGameMode (Game|GetGameMode)))
  (Variables|Default|SetGameModeRef _asbp_runner_game_mode))

(event Input|TouchEvents|InputTouch
  (params (Location :type Vector) (FingerIndex :type ETouchIndex%20Enum))
  (bind _returnvalue (Math|Vector2D|MakeVector2D (.x Location) (.y Location)))
  (:Pressed
    (Variables|Touch|SetisActive true)
    (Variables|Touch|SetTouch_Start_Position _returnvalue))
  (:Released
    (Variables|Touch|SetisActive false)
    (Math|Integer|IncrementInt (Variables|Touch|GetClickCout)
      (:%20%20
        (if (>= (Variables|Touch|GetClickCout) 2)
          (Default|DoubleClick (Variables|Default|GetPlayerRef))
          (else
            (Utilities|FlowControl|Delay 0.5)))
        (Variables|Touch|SetClickCout 0))))
  (:Moved
    (if (and (Variables|Touch|GetisActive) (Variables|/Game/Runner/Blueprints/BP_RunnerGameMode.BP_RunnerGameMode_C|GetIsGameStarted (Variables|Default|GetGameModeRef)))
      (Variables|Touch|SetTouch_Current_Position _returnvalue)
      (Utilities|FlowControl|Sequence
        (:then_0
          (if (> (.x (- (Variables|Touch|GetTouch_Start_Position) (Variables|Touch|GetTouch_Current_Position))) (Variables|Touch|GetTouchThresHold))
            (Variables|Touch|SetisActive false)
            (Default|SwipLeft (Variables|Default|GetPlayerRef))
            (Variables|Touch|SetClickCout 0 :!label _label)))
        (:then_1
          (if (< (.x (- (Variables|Touch|GetTouch_Start_Position) (Variables|Touch|GetTouch_Current_Position))) (* (Variables|Touch|GetTouchThresHold) -1.0))
            (Variables|Touch|SetisActive false)
            (Default|SwipRight (Variables|Default|GetPlayerRef))
            (goto _label)))
        (:then_2
          (if (> (.y (- (Variables|Touch|GetTouch_Start_Position) (Variables|Touch|GetTouch_Current_Position))) (Variables|Touch|GetTouchThresHold))
            (Variables|Touch|SetisActive false)
            (Default|SwipUp (Variables|Default|GetPlayerRef))
            (goto _label)))
        (:then_3
          (if (< (.y (- (Variables|Touch|GetTouch_Start_Position) (Variables|Touch|GetTouch_Current_Position))) (* (Variables|Touch|GetTouchThresHold) -1.0))
            (Variables|Touch|SetisActive false)
            (Default|SwipDown (Variables|Default|GetPlayerRef))
            (goto _label)))))))

(fn ConstructionScript)