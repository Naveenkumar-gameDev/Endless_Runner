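; Runner game camera that follows the player's spawn-point component each tick, at fixed height unless a jump boost lifts the player high.
; Lane-offset interpolation receives zero delta time, so Y simply tracks that component.
; Player forward speed drives speed-line effect alpha and smoothly widens field of view.
; On death, the camera eases to a narrower view and rotates toward the player's mesh.
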(event Collision|EventActorBeginOverlap
  (params (OtherActor :type Actor%20Object%20Reference)))

(event EventTick
  (params (DeltaSeconds :type Float%20%28single-precision%29))
  (Utilities|FlowControl|Sequence
    (:then_0
      (CallFunction|FollowPlayer 0.0)
      (CallFunction|ShowEfforts))
    (:then_1
      (if (Variables|/Game/Runner/Blueprints/BP_RunnerCharacter.BP_RunnerCharacter_C|GetisDead (Variables|Default|GetPlaye_Ref))
        (CallFunction|DeathCameraEffect)
        (else
          (CallFunction|SetCamaraView))))))

(fn ConstructionScript)

(fn FollowPlayer
  (params (Delta :type Float%20%28double-precision%29))
  (bind _playe_ref (Variables|Default|GetPlaye_Ref))
  (bind (_x _y _z) (CallFunction|GetCameraLocation Delta))
  (bind (_x_2 _y_2) (CallFunction|GetCameraLocation Delta))
  (bind _capsulecomponent (Variables|/Script/Engine.Character|GetCapsuleComponent _playe_ref))
  (bind _returnvalue (Transformation|GetWorldLocation _capsulecomponent))
  (if (not (Variables|/Game/Runner/Blueprints/BP_RunnerCharacter.BP_RunnerCharacter_C|GetIsJumbBoostEnable _playe_ref))
    (Transformation|SetActorLocation (Math|Vector|MakeVector _x _y _z) false false :!label _label)
    (elif (not (> (.z _returnvalue) 2.1e+02))
      (goto _label)
      (else
        (Transformation|SetActorLocation (Math|Vector|MakeVector _x_2 _y_2 (- (.z _returnvalue) 5e+01)) false false)))))

(fn GetCameraLocation
  (params (Delta :type Float%20%28double-precision%29))
  (bind _playe_ref (Variables|Default|GetPlaye_Ref))
  (bind _cameraspawnpoint (Variables|/Game/Runner/Blueprints/BP_RunnerCharacter.BP_RunnerCharacter_C|GetCameraSpawnPoint _playe_ref))
  (bind _returnvalue (Transformation|GetWorldLocation _cameraspawnpoint))
  (return (.x _returnvalue) (Math|Interpolation|FInterpTo (.y _returnvalue) (* (- (Variables|/Game/Runner/Blueprints/BP_RunnerCharacter.BP_RunnerCharacter_C|GetCurrentLane _playe_ref) 1) (Variables|Default|GetLaneOffSet)) Delta 1.0) (Variables|Default|GetStartZVal)))

(fn ShowEfforts
  (Niagara|SetNiagaraVariable(LinearColor) (Variables|Default|GetSpeedEffort) "Scale Value" (Utilities|Struct|MakeLinearColor 1.0 1.0 1.0 (Math|Float|MapRangeClamped (.x (Transformation|GetVelocity (Variables|Default|GetPlaye_Ref))) (Variables|Default|GetSpeedLineStartVal) (Variables|Default|GetSpeedLineEndVal) 0.0 1.0))))

(fn SetCamaraView
  (Camera|SetFieldOfView (Variables|Default|GetCamera) (Math|Interpolation|FInterpTo (Variables|/Script/Engine.CameraComponent|GetFieldOfView (Variables|Default|GetCamera)) (Math|Float|MapRangeClamped (.x (Transformation|GetVelocity (Variables|Default|GetPlaye_Ref))) 6e+02 1.5e+03 9e+01 1.2e+02) (Utilities|Time|GetWorldDeltaSeconds) 3.0)))

(fn DeathCameraEffect
  (bind _camera (Variables|Default|GetCamera))
  (Camera|SetFieldOfView _camera (Math|Interpolation|FInterpTo (Variables|/Script/Engine.CameraComponent|GetFieldOfView (Variables|Default|GetCamera)) 7e+01 (Utilities|Time|GetWorldDeltaSeconds) 1.0))
  (Transformation|SetWorldRotation (Variables|Default|GetCamera) (Math|Interpolation|RInterpTo (Transformation|GetWorldRotation _camera) (Math|Rotator|FindLookatRotation (Transformation|GetWorldLocation _camera) (Transformation|GetWorldLocation (Variables|/Script/Engine.Character|GetMesh (Variables|Default|GetPlaye_Ref)))) (Utilities|Time|GetWorldDeltaSeconds) 7.0) false false))