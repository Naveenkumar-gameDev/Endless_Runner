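; Game mode for a three-lane endless runner that manages music, start screen, HUD, distance-based score and coin total.
; BeginPlay lays the first tiles and shows the start widget; Start switches music, adds the HUD and starts the player.
; SpawnTile chains tiles by their spawn points, triggers building spawns and fills obstacle spawners with random child actors in random lanes.
; A looping timer periodically re-enables power spawns, each consuming the flag.
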(event Custom|Start
  (bind _audioplayer (Variables|Default|GetAudioPlayer))
  (bind _audiocomponent (Variables|/Script/Engine.AmbientSound|GetAudioComponent _audioplayer))
  (Audio|Components|Audio|SetSound _audiocomponent "/Game/Runner/Audios/GamePlay_Music.GamePlay_Music")
  (Audio|Components|Audio|Play _audiocomponent 0.0)
  (bind _returnvalue (UserInterface|CreateWidget "/Game/Runner/Blueprints/HUD/HUD_Player.HUD_Player_C"))
  (bind _output_get (Variables|Default|SetHUD_Ref _returnvalue))
  (UserInterface|Viewport|AddtoViewport _output_get 0)
  (Variables|/Game/Runner/Blueprints/BP_RunnerCharacter.BP_RunnerCharacter_C|SetHUD_Player_Ref (Variables|Default|GetPlayer_Ref) (Variables|Default|GetHUD_Ref))
  (Default|Start (Variables|Default|GetPlayer_Ref))
  (Utilities|FlowControl|Delay 1.0)
  (Variables|Default|SetIsGameStarted true))

(event EventBeginPlay
  (bind _audioplayer (Variables|Default|GetAudioPlayer))
  (bind _audiocomponent (Variables|/Script/Engine.AmbientSound|GetAudioComponent _audioplayer))
  (Utilities|FlowControl|DelayUntilNextTick)
  (Audio|Components|Audio|SetSound _audiocomponent "/Game/Runner/Audios/background_Music_New.background_Music_New")
  (Audio|Components|Audio|Play _audiocomponent 0.0)
  (bind _returnvalue (Actor|GetActorOfClass "/Game/Runner/Blueprints/BP_RunnerCharacter.BP_RunnerCharacter_C"))
  (Variables|Default|SetPlayer_Ref _returnvalue)
  (CallFunction|SpawnTile 5)
  (bind _returnvalue_2 (UserInterface|CreateWidget "/Game/Runner/Blueprints/HUD/WB_GameStart.WB_GameStart_C" 0 self))
  (UserInterface|Viewport|AddtoViewport _returnvalue_2 0)
  (Utilities|Time|SetTimerbyFunctionName 0 "SetCanSpawnTrue" 2e+01 true))

(event EventTick
  (params (DeltaSeconds :type Float%20%28single-precision%29))
  (if (Variables|Default|GetIsGameStarted)
    (Variables|Default|SetPlayer_Score (Math|Float|Truncate (/ (.x (Transformation|GetWorldLocation (Variables|/Script/Engine.Character|GetCapsuleComponent (Variables|Default|GetPlayer_Ref)))) 1e+01)))
    (Default|ShowPoints (Variables|Default|GetHUD_Ref) (Variables|Default|GetPlayer_Score))))

(fn ConstructionScript)

(fn SpawnTile
  (params (SpawnCount :type Integer))
  (for _index (range 1 SpawnCount)
    (bind _returnvalue (Game|SpawnActorfromClass "/Game/Runner/Blueprints/Others/BP_BaseTile.BP_BaseTile_C" (Math|Transform|MakeTransform (Variables|Default|GetTile_SpawnPoint) "0, 0, 0" "1.000000,1.000000,1.000000") "Undefined" "MultiplyWithRoot" 0 0))
    (bind _output_get (Variables|Default|SetTile_Ref _returnvalue))
    (Variables|Default|SetTile_SpawnPoint (Transformation|GetWorldLocation (Variables|/Game/Runner/Blueprints/Others/BP_BaseTile.BP_BaseTile_C|GetSpawnPoint _output_get)))
    (Variables|/Game/Runner/Blueprints/Others/BP_BaseTile.BP_BaseTile_C|SetGameMode_Ref _output_get self)
    (CallFunction|SpawnObstacle)
    (for _array_element (Variables|Default|GetSpawnBuilding_Ref)
      (Default|SpawnBuilding _array_element))))

(fn SpawnObstacle
  (bind _tile_ref (Variables|Default|GetTile_Ref))
  (for _array_element (Components|GetChildrenComponents (Variables|/Game/Runner/Blueprints/Others/BP_BaseTile.BP_BaseTile_C|GetObstacleSpawners _tile_ref) false)
    (switch int (Math|Random|RandomInteger 4)
      (:0
        (AddComponent|AddChildActorComponent _tile_ref false (Math|Transform|MakeTransform (Math|Vector|MakeVector (.x (Variables|/Script/Engine.SceneComponent|GetRelativeLocation _array_element)) (+ (.y (Variables|/Script/Engine.SceneComponent|GetRelativeLocation _array_element)) (Utilities|Select :Index (Math|Random|RandomInteger 3) :Option%200 2.2e+02 :Option%201 0.0 :Option%202 -2.2e+02)) (.z (Variables|/Script/Engine.SceneComponent|GetRelativeLocation _array_element))) "0, 0, 0" "1.000000,1.000000,1.000000")))
      (:1
        (AddComponent|AddChildActorComponent _tile_ref false (Math|Transform|MakeTransform (Math|Vector|MakeVector (.x (Variables|/Script/Engine.SceneComponent|GetRelativeLocation _array_element)) (+ (.y (Variables|/Script/Engine.SceneComponent|GetRelativeLocation _array_element)) (Utilities|Select :Index (Math|Random|RandomInteger 3) :Option%200 2.2e+02 :Option%201 0.0 :Option%202 -2.2e+02)) (.z (Variables|/Script/Engine.SceneComponent|GetRelativeLocation _array_element))) "0, 0, 0" "1.000000,1.000000,1.000000")))
      (:2
        (AddComponent|AddChildActorComponent _tile_ref false (Math|Transform|MakeTransform (Math|Vector|MakeVector (.x (Variables|/Script/Engine.SceneComponent|GetRelativeLocation _array_element)) (+ (.y (Variables|/Script/Engine.SceneComponent|GetRelativeLocation _array_element)) (Utilities|Select :Index (Math|Random|RandomInteger 3) :Option%200 2.2e+02 :Option%201 0.0 :Option%202 -2.2e+02)) (.z (Variables|/Script/Engine.SceneComponent|GetRelativeLocation _array_element))) "0, 0, 0" "1.000000,1.000000,1.000000")))
      (:3
        (if (not (Variables|Default|GetCanSpawnPower))
          (for _index (range 0 (Math|Random|RandomIntegerinRange 0 4))
            (AddComponent|AddChildActorComponent _tile_ref false (Math|Transform|MakeTransform (Math|Vector|MakeVector (+ (.x (Variables|/Script/Engine.SceneComponent|GetRelativeLocation _array_element)) (* _index 200)) (+ (.y (Variables|/Script/Engine.SceneComponent|GetRelativeLocation _array_element)) (Utilities|Select :Index (Math|Random|RandomInteger 3) :Option%200 2.2e+02 :Option%201 0.0 :Option%202 -2.2e+02)) (.z (Variables|/Script/Engine.SceneComponent|GetRelativeLocation _array_element))) "0, 0, 0" "1.000000,1.000000,1.000000")))
          (else
            (Variables|Default|SetCanSpawnPower false)
            (switch int (Math|Random|RandomIntegerinRange 0 1)
              (:0
                (AddComponent|AddChildActorComponent _tile_ref false (Math|Transform|MakeTransform (Math|Vector|MakeVector (+ (.x (Variables|/Script/Engine.SceneComponent|GetRelativeLocation _array_element)) (* _index 200)) (+ (.y (Variables|/Script/Engine.SceneComponent|GetRelativeLocation _array_element)) (Utilities|Select :Index (Math|Random|RandomInteger 3) :Option%200 2.2e+02 :Option%201 0.0 :Option%202 -2.2e+02)) 115.0) "0, 0, 0" "1.000000,1.000000,1.000000")))
              (:1
                (AddComponent|AddChildActorComponent _tile_ref false (Math|Transform|MakeTransform (Math|Vector|MakeVector (+ (.x (Variables|/Script/Engine.SceneComponent|GetRelativeLocation _array_element)) (* _index 200)) (+ (.y (Variables|/Script/Engine.SceneComponent|GetRelativeLocation _array_element)) (Utilities|Select :Index (Math|Random|RandomInteger 3) :Option%200 2.2e+02 :Option%201 0.0 :Option%202 -2.2e+02)) 115.0) "0, 0, 0" "1.000000,1.000000,1.000000"))))))))))

(fn IncreaseCoins
  (params (Points :type Integer))
  (bind _output_get (Variables|Default|SetCoins (+ Points (Variables|Default|GetCoins))))
  (Default|ShowCoins (Variables|Default|GetHUD_Ref) _output_get))

(fn SetCanSpawnTrue
  (Variables|Default|SetCanSpawnPower true))